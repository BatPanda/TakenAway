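; AI enemy that spots, chases and shoots the player, starting with a dev pistol.
; Each tick it updates inherited movement and sprites, then fires a horizontal ring of 360 line traces to find the player.
; With sight it turns its body and attacks through a timer-reset cooldown gate; after losing sight it pursues with AIMoveTo.
; Only the pistol attack is implemented, spawning a projectile aimed at the player.
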(event `self.ReceiveBeginPlay`
  (set `self.IsAi` true)
  (set `self.WeaponEquipped` "NewEnumerator3")
  (set `self.WeaponData` (make `/Game/Blueprints/Core/WeaponInfo` 10 10)))

(event `self.ReceiveTick`
  (params (DeltaSeconds :type "Float (single-precision)"))
  (if (not (`self.Dead`))
    (`self.MovementUpdate`)
    (`self.HandleSprites`)
    (bind _found (`self.LookForPlayer`))
    (bind _output_get (set `self.CanSeePlayer` _found))
    (if _output_get
      (set `self.PlayerDetected` true))
    (if (`self.CanSeePlayer`)
      (`self.FacePlayer`)
      (`/Engine/EditorBlueprintResources/StandardMacros.Gate` false :!label _label
        (:`Exit`
          (`self.AttackPlayer`)
          (`KismetSystemLibrary.K2_SetTimerDelegate` (delegate `ResetCooldown`) (select `/Game/Blueprints/Core/Weapons` (`self.WeaponEquipped`) :`NewEnumerator3` 0.6 :!type "Float (single-precision)"))
          (goto _label :!via `Close`)))
      (elif (`self.PlayerDetected`)
        (`|AIMoveTo` self (0.0 0.0 0.0) (`GameplayStatics.GetPlayerCharacter` 0) (select `/Game/Blueprints/Core/Weapons` (`self.WeaponEquipped`) :`NewEnumerator3` 200.0 :!type "Float (single-precision)")
          (:`OnSuccess`
            (goto _label)))))))

(event `ResetCooldown`
  (goto _label :!via `Open`))

(fn `AttackPlayer`
  (bind (_weapondata_currentammo _weapondata_maxammo) (break `/Game/Blueprints/Core/WeaponInfo` (`self.WeaponData`)))
  (bind _returnvalue (`SceneComponent.K2_GetComponentToWorld` (`self.FirePoint`)))
  (if (or (== _weapondata_maxammo -1) (> _weapondata_currentammo 0))
    (switch `/Game/Blueprints/Core/Weapons` (`self.WeaponEquipped`)
      (:`NewEnumerator3`
        (bind _unit_vec (`self.GetLineFromAIToPlayer`))
        (bind _returnvalue_2 (`|SpawnActorFromClass` "/Game/Blueprints/Actors/bullet.bullet_C" (`KismetMathLibrary.MakeTransform` (`KismetMathLibrary.MakeVector` (.x (.location _returnvalue)) (.y (.location _returnvalue)) (+ (.z (.location _returnvalue)) 20.0)) (.rotation _returnvalue)) "Undefined" "OverrideRootScale" null null))
        (set `MovementComponent.Velocity` (* _unit_vec 800.0) (`/Game/Blueprints/Actors/bullet.ProjectileMovement` _returnvalue_2))))))

(fn `FacePlayer`
  (bind _returnvalue_roll (`KismetMathLibrary.BreakRotator` (`self.K2_GetActorRotation`)))
  (bind (_returnvalue_roll_2 _returnvalue_pitch _returnvalue_yaw) (`KismetMathLibrary.BreakRotator` (`KismetMathLibrary.FindLookAtRotation` (`self.K2_GetActorLocation`) (`self.K2_GetActorLocation` (cast `/Game/Blueprints/Actors/TakenMainCharacter` (`GameplayStatics.GetPlayerCharacter` 0) :!pure true)))))
  (`SceneComponent.K2_SetWorldRotation` (`self.Body`) (`KismetMathLibrary.MakeRotator` (- _returnvalue_roll 90.0) 0.0 (+ _returnvalue_yaw 90.0)) false false))

(fn `GetLineFromAIToPlayer`
  (returns (`Unit Vec` :type "Vector Structure"))
  (bind (_returnvalue_x _returnvalue_y) (`KismetMathLibrary.BreakVector` (`self.K2_GetActorLocation`)))
  (bind (_returnvalue_x_2 _returnvalue_y_2) (`KismetMathLibrary.BreakVector` (`self.K2_GetActorLocation` (cast `/Game/Blueprints/Actors/TakenMainCharacter` (`GameplayStatics.GetPlayerCharacter` 0) :!pure true))))
  (return (`KismetMathLibrary.GetDirectionUnitVector` (`KismetMathLibrary.MakeVector` _returnvalue_x _returnvalue_y) (`KismetMathLibrary.MakeVector` _returnvalue_x_2 _returnvalue_y_2))))

(fn `LookForPlayer`
  (returns (Found :type Boolean))
  (locals (`Found Player` :type Boolean))
  (for _index (range 1 361)
    (bind _returnvalue (`KismetMathLibrary.Conv_IntToDouble` _index))
    (bind _found (`self.RaycastCheckForPlayer` (`KismetMathLibrary.MakeVector` (* 600.0 (`KismetMathLibrary.Cos` _returnvalue)) (* 600.0 (`KismetMathLibrary.Sin` _returnvalue)))))
    (if _found
      (set `local.Found Player` true)))
  (return (`local.Found Player`)))

(fn `RaycastCheckForPlayer`
  (params (Vec :type "Vector Structure"))
  (returns (Found :type Boolean))
  (bind _returnvalue (`self.K2_GetActorLocation`))
  (bind _outhit (`KismetSystemLibrary.LineTraceSingleForObjects` _returnvalue (+ _returnvalue Vec) (`|MakeArray` "ObjectTypeQuery3" "ObjectTypeQuery1" :!type "EObjectTypeQuery Enum")))
  (bind (_bblockinghit _binitialoverlap _time _distance _location _impactpoint _normal _impactnormal _physmat _hitactor) (`GameplayStatics.BreakHitResult` _outhit))
  (cast `/Game/Blueprints/Actors/Enemy` _hitactor
    (:`CastFailed`
      (cast `/Game/Blueprints/Actors/TakenMainCharacter` _hitactor
        (:`then`
          (return true))
        (:`CastFailed`
          (return false))))))

(fn `UserConstructionScript`
  (`parent.UserConstructionScript`))