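; Top-down flipbook character with an IsAi switch for player or AI, handling movement, weapons and bullet deaths.
; Separate body and leg sprites follow cursor aim (player only) and movement direction.
; Attacks punch or fire pistol and shotgun bullets; weapons can be picked up and thrown, including when empty.
; Player movement drives global time dilation, offset by custom dilation, and a death leaving no living enemies loads the next level.
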(event `InputAxis|MoveForward`
  (params (AxisValue :type "Float (single-precision)"))
  (if (not (`self.Dead`))
    (set `self.IsMoving` false)
    (`self.AddMovementInput` (1.0 0.0 0.0) AxisValue)
    (set `self.IsMoving` false)))

(event `InputAxis|MoveRight`
  (params (AxisValue :type "Float (single-precision)"))
  (if (not (`self.Dead`))
    (set `self.IsMoving` false)
    (`self.AddMovementInput` (0.0 1.0 0.0) AxisValue)
    (set `self.IsMoving` false)))

(event `self.ReceiveTick`
  (params (DeltaSeconds :type "Float (single-precision)"))
  (if (not (`self.Dead`))
    (`self.MovementUpdate`)
    (`self.HandleSprites`)
    (if (`self.IsAi`)
      _
      (elif (`self.IsMoving`)
        (`self.ChangeSpeed` true)
        (else
          (`self.ChangeSpeed` false))))))

(event `InputAction|Throw/Pickup`
  (params (Key :type "Key Structure"))
  (:`Pressed`
    (if (`self.Dead`)
      _
      (elif (`|EnumEquality` (`self.WeaponEquipped`) "NewEnumerator0")
        (if (`self.InRangeOfWeapon`)
          (`self.PickupWeapon`))
        (else
          (`self.ThrowWeapon`))))))

(event `InputAction|Fire/Swing`
  (params (Key :type "Key Structure"))
  (:`Pressed`
    (if (not (`self.Dead`))
      (`/Engine/EditorBlueprintResources/StandardMacros.Gate` false :!label _label
        (:`Exit`
          (`self.Attack`)
          (`KismetSystemLibrary.K2_SetTimerDelegate` (delegate `ResetWeapon`) (select `/Game/Blueprints/Core/Weapons` (`self.WeaponEquipped`) :`NewEnumerator0` 0.1 :`NewEnumerator1` 0.1 :`NewEnumerator2` 0.6 :`NewEnumerator3` 0.6 :!type "Float (single-precision)"))
          (goto _label :!via `Close`))))))

(event `ResetWeapon`
  (goto _label :!via `Open`))

(event `self.Box.OnComponentBeginOverlap`
  (params (OverlappedComponent :type "PrimitiveComponent Object Reference") (OtherActor :type "Actor Object Reference") (OtherComp :type "PrimitiveComponent Object Reference") (OtherBodyIndex :type Integer) (bFromSweep :type Boolean) (SweepResult :type "HitResult Structure (by ref)"))
  (bind _asbullet (cast `/Game/Blueprints/Actors/bullet` OtherActor))
  (if (`self.Dead`)
    _
    (elif (`self.IsAi`)
      (bind _friendly (`/Game/Blueprints/Actors/bullet.Friendly` _asbullet))
      (if _friendly
        (bind _gameend (`self.Die` :!label _label_2))
        (bind _output_get (set `self.Complete` _gameend))
        (if _output_get
          (`GameplayStatics.OpenLevel` (`/Game/Blueprints/Core/CoreInstance.NextLevel` (cast `/Game/Blueprints/Core/CoreInstance` (`GameplayStatics.GetGameInstance`) :!pure true)))
          (else
            (`self.K2_DestroyActor` _asbullet))))
      (elif (not _friendly)
        (goto _label_2)))))

(event `InputAction|Reset`
  (params (Key :type "Key Structure"))
  (:`Pressed`
    (`GameplayStatics.OpenLevel` (`/Game/Blueprints/Core/CoreInstance.CurrentLevel` (cast `/Game/Blueprints/Core/CoreInstance` (`GameplayStatics.GetGameInstance`) :!pure true)))))

(fn `Attack`
  (bind (_weapondata_currentammo _weapondata_maxammo) (break `/Game/Blueprints/Core/WeaponInfo` (`self.WeaponData`)))
  (bind _body (`self.Body`))
  (bind (_weapondata_currentammo_2 _weapondata_maxammo_2) (break `/Game/Blueprints/Core/WeaponInfo` (`self.WeaponData`)))
  (bind (_weapondata_currentammo_3 _weapondata_maxammo_3) (break `/Game/Blueprints/Core/WeaponInfo` (`self.WeaponData`)))
  (bind (_returnvalue_location _returnvalue_rotation) (`KismetMathLibrary.BreakTransform` (`SceneComponent.K2_GetComponentToWorld` (`self.FirePoint`))))
  (bind (_returnvalue_location_2 _returnvalue_rotation_2) (`KismetMathLibrary.BreakTransform` (`SceneComponent.K2_GetComponentToWorld` (`self.ShotGunFP`))))
  (if (or (== _weapondata_maxammo -1) (> _weapondata_currentammo 0))
    (switch `/Game/Blueprints/Core/Weapons` (`self.WeaponEquipped`)
      (:`NewEnumerator0`
        (set `self.IsPunching` true)
        (`PaperFlipbookComponent.SetPlayRate` _body 0.0)
        (`PaperFlipbookComponent.SetFlipbook` _body "/Game/Sprites/Useful/RedPunch.RedPunch"))
      (:`NewEnumerator2`
        (bind _unit_vec (`self.GetLineFromCharToMouse`))
        (bind _returnvalue (`|SpawnActorFromClass` "/Game/Blueprints/Actors/bullet.bullet_C" (`KismetMathLibrary.MakeTransform` _returnvalue_location_2 _returnvalue_rotation_2) "Undefined" "OverrideRootScale" null true null))
        (bind _returnvalue_2 (* (+ (* (`KismetMathLibrary.Cross_VectorVector` _unit_vec (0.0 0.0 1.0)) (`KismetMathLibrary.RandomFloatInRange` -0.2 0.2)) _unit_vec) 1800.0))
        (set `MovementComponent.Velocity` _returnvalue_2 (`/Game/Blueprints/Actors/bullet.ProjectileMovement` _returnvalue))
        (bind _returnvalue_3 (`|SpawnActorFromClass` "/Game/Blueprints/Actors/bullet.bullet_C" (`KismetMathLibrary.MakeTransform` _returnvalue_location_2 _returnvalue_rotation_2) "Undefined" "OverrideRootScale" null true null))
        (set `MovementComponent.Velocity` _returnvalue_2 (`/Game/Blueprints/Actors/bullet.ProjectileMovement` _returnvalue_3))
        (bind _returnvalue_4 (`|SpawnActorFromClass` "/Game/Blueprints/Actors/bullet.bullet_C" (`KismetMathLibrary.MakeTransform` _returnvalue_location_2 _returnvalue_rotation_2) "Undefined" "OverrideRootScale" null true null))
        (set `MovementComponent.Velocity` _returnvalue_2 (`/Game/Blueprints/Actors/bullet.ProjectileMovement` _returnvalue_4))
        (bind _returnvalue_5 (`|SpawnActorFromClass` "/Game/Blueprints/Actors/bullet.bullet_C" (`KismetMathLibrary.MakeTransform` _returnvalue_location_2 _returnvalue_rotation_2) "Undefined" "OverrideRootScale" null true null))
        (set `MovementComponent.Velocity` _returnvalue_2 (`/Game/Blueprints/Actors/bullet.ProjectileMovement` _returnvalue_5))
        (bind _returnvalue_6 (`|SpawnActorFromClass` "/Game/Blueprints/Actors/bullet.bullet_C" (`KismetMathLibrary.MakeTransform` _returnvalue_location_2 _returnvalue_rotation_2) "Undefined" "OverrideRootScale" null true null))
        (set `MovementComponent.Velocity` _returnvalue_2 (`/Game/Blueprints/Actors/bullet.ProjectileMovement` _returnvalue_6))
        (set `self.WeaponData` (make `/Game/Blueprints/Core/WeaponInfo` (- _weapondata_currentammo_2 1) _weapondata_maxammo_2)))
      (:`NewEnumerator3`
        (bind _unit_vec_2 (`self.GetLineFromCharToMouse`))
        (bind _returnvalue_7 (`|SpawnActorFromClass` "/Game/Blueprints/Actors/bullet.bullet_C" (`KismetMathLibrary.MakeTransform` _returnvalue_location _returnvalue_rotation) "Undefined" "OverrideRootScale" null true null))
        (set `MovementComponent.Velocity` (* _unit_vec_2 1800.0) (`/Game/Blueprints/Actors/bullet.ProjectileMovement` _returnvalue_7))
        (set `self.WeaponData` (make `/Game/Blueprints/Core/WeaponInfo` (- _weapondata_currentammo_3 1) _weapondata_maxammo_3))))
    (elif (not (`|EnumEquality` (`self.WeaponEquipped`) "NewEnumerator0"))
      (`self.ThrowWeapon`))))

(fn `BodyMovement`
  (bind _returnvalue_roll (`KismetMathLibrary.BreakRotator` (`self.K2_GetActorRotation`)))
  (bind (_returnvalue_roll_2 _returnvalue_pitch _returnvalue_yaw) (`KismetMathLibrary.BreakRotator` (`KismetMathLibrary.FindLookAtRotation` (`self.K2_GetActorLocation`) (`.Location` (`GameplayStatics.BreakHitResult` (`PlayerController.GetHitResultUnderCursorByChannel` (`GameplayStatics.GetPlayerController` 0) "TraceTypeQuery2" true))))))
  (`SceneComponent.K2_SetWorldRotation` (`self.Body`) (`KismetMathLibrary.MakeRotator` (- _returnvalue_roll 90.0) 0.0 (+ _returnvalue_yaw 90.0)) false false))

(fn `BodySpriteUpdate`
  (bind _weaponequipped (`self.WeaponEquipped`))
  (if (not (`self.IsPunching`))
    (`PaperFlipbookComponent.SetFlipbook` (`self.Body`) (select `bool` (`self.IsAi`) :`false` (select `/Game/Blueprints/Core/Weapons` _weaponequipped :`NewEnumerator0` "/Game/Sprites/Useful/RedBody.RedBody" :`NewEnumerator1` "/Game/Sprites/Useful/RedBodyKnife.RedBodyKnife" :`NewEnumerator2` "/Game/Sprites/Useful/Red_Body_Armed_Shotgun.Red_Body_Armed_Shotgun" :`NewEnumerator3` "/Game/Sprites/Useful/RedBodyPistol.RedBodyPistol" :!type "PaperFlipbook Object Reference") :`true` (select `/Game/Blueprints/Core/Weapons` _weaponequipped :`NewEnumerator0` "/Game/Sprites/Useful/BlueBody.BlueBody" :`NewEnumerator1` "/Game/Sprites/Useful/BlueBodyKnife.BlueBodyKnife" :`NewEnumerator2` "/Game/Sprites/Useful/BlueBodyShotgun.BlueBodyShotgun" :`NewEnumerator3` "/Game/Sprites/Useful/BlueBodyPistol.BlueBodyPistol" :!type "PaperFlipbook Object Reference")))))

(fn `ChangeSpeed`
  (params (Increase :type Boolean))
  (bind _returnvalue (`GameplayStatics.GetGlobalTimeDilation`))
  (bind _returnvalue_2 (* (`GameplayStatics.GetWorldDeltaSeconds`) 10.0))
  (if Increase
    (`GameplayStatics.SetGlobalTimeDilation` (`KismetMathLibrary.FClamp` (+ _returnvalue _returnvalue_2) 0.01 0.5))
    (else
      (`GameplayStatics.SetGlobalTimeDilation` (`KismetMathLibrary.FClamp` (- _returnvalue _returnvalue_2) 0.01 0.5))))
  (set `self.CustomTimeDilation` (/ 1.0 (`GameplayStatics.GetGlobalTimeDilation`))))

(fn `Die`
  (returns (GameEnd :type Boolean))
  (locals (GameOver :type Boolean :default true))
  (bind (_returnvalue_x _returnvalue_y) (`KismetMathLibrary.BreakVector` (`self.K2_GetActorLocation`)))
  (if (not (`self.Dead`))
    (set `self.Dead` true)
    (`PaperFlipbookComponent.SetFlipbook` (`self.Head`) (select `bool` (`self.IsAi`) :`false` "/Game/Sprites/Useful/RedDead.RedDead" :`true` "/Game/Sprites/Useful/BlueDead.BlueDead" :!type "PaperFlipbook Object Reference"))
    (`PaperFlipbookComponent.SetFlipbook` (`self.Body`) null)
    (`PaperFlipbookComponent.SetFlipbook` (`self.Sprite`) null)
    (`NavMovementComponent.StopActiveMovement` (`self.CharacterMovement`))
    (`PrimitiveComponent.SetCollisionEnabled` (`self.CapsuleComponent`) "NoCollision")
    (`self.K2_SetActorLocation` (`KismetMathLibrary.MakeVector` _returnvalue_x _returnvalue_y 51.0) false true)
    (bind _outactors (`GameplayStatics.GetAllActorsOfClass` "/Game/Blueprints/Actors/Enemy.Enemy_C"))
    (for _array_element _outactors
      (if (not (`/Game/Blueprints/Actors/TakenMainCharacter.Dead` _array_element))
        (set `local.GameOver` false)))
    (if (`local.GameOver`)
      (return true)
      (else
        (return false)))))

(fn `GetLineFromCharToMouse`
  (returns (`Unit Vec` :type "Vector Structure"))
  (bind (_returnvalue_x _returnvalue_y) (`KismetMathLibrary.BreakVector` (`self.K2_GetActorLocation`)))
  (bind (_bblockinghit _binitialoverlap _time _distance _location) (`GameplayStatics.BreakHitResult` (`PlayerController.GetHitResultUnderCursorByChannel` (`GameplayStatics.GetPlayerController` 0) "TraceTypeQuery2" true)))
  (return (`KismetMathLibrary.GetDirectionUnitVector` (`KismetMathLibrary.MakeVector` _returnvalue_x _returnvalue_y) (`KismetMathLibrary.MakeVector` (.x _location) (.y _location)))))

(fn `HandleSprites`
  (`self.LegVisability`)
  (`self.BodySpriteUpdate`)
  (if (not (`self.IsAi`))
    (`self.BodyMovement`))
  (`self.LegRotation`))

(fn `LegRotation`
  (`SceneComponent.K2_SetWorldRotation` (`self.Sprite`) (`KismetMathLibrary.MakeRotator` -90.0 0.0 (+ (select `/Game/Blueprints/Core/MovementDirection` (`self.MovementDirection`) :`NewEnumerator1` 90.0 :`NewEnumerator2` 180.0 :`NewEnumerator3` 270.0 :`NewEnumerator4` 45.0 :`NewEnumerator5` 135.0 :`NewEnumerator6` 225.0 :`NewEnumerator7` 315.0 :!type "Float (single-precision)") 90.0)) false false))

(fn `LegVisability`
  (`PaperFlipbookComponent.SetFlipbook` (`self.Sprite`) (select `bool` (`self.IsMoving`) :`true` "/Game/Sprites/Useful/RedWalk.RedWalk" :!type "PaperFlipbook Object Reference")))

(fn `MovementUpdate`
  (locals (MovementVector :type "Vector2D Structure"))
  (bind _returnvalue (`self.GetInputAxisValue`))
  (bind _returnvalue_2 (`self.GetInputAxisValue`))
  (bind _returnvalue_3 (`self.GetInputAxisValue`))
  (bind _returnvalue_4 (`self.GetInputAxisValue`))
  (if (and (== _returnvalue_3 0.0) (== _returnvalue_4 0.0))
    (set `self.IsMoving` false)
    (else
      (set `self.IsMoving` true)
      (if (and (== _returnvalue_3 1.0) (== _returnvalue_4 0.0))
        (set `self.MovementDirection` "NewEnumerator0")
        (elif (and (== _returnvalue_3 -1.0) (== _returnvalue_4 0.0))
          (set `self.MovementDirection` "NewEnumerator2")
          (elif (and (== _returnvalue_3 0.0) (== _returnvalue_4 1.0))
            (set `self.MovementDirection` "NewEnumerator1")
            (elif (and (== _returnvalue_3 0.0) (== _returnvalue_4 -1.0))
              (set `self.MovementDirection` "NewEnumerator3")
              (elif (and (== _returnvalue 1.0) (== _returnvalue_2 1.0))
                (set `self.MovementDirection` "NewEnumerator4")
                (elif (and (== _returnvalue 1.0) (== _returnvalue_2 -1.0))
                  (set `self.MovementDirection` "NewEnumerator7")
                  (elif (and (== _returnvalue -1.0) (== _returnvalue_2 1.0))
                    (set `self.MovementDirection` "NewEnumerator5")
                    (else
                      (set `self.MovementDirection` "NewEnumerator6"))))))))))))

(fn `PickupWeapon`
  (bind _weapontopickup (`self.WeaponToPickUp`))
  (set `self.WeaponEquipped` (`/Game/Blueprints/Actors/Weapon.Type` _weapontopickup))
  (set `self.WeaponData` (`/Game/Blueprints/Actors/Weapon.Data` _weapontopickup))
  (`self.K2_DestroyActor` (`self.WeaponToPickUp`)))

(fn `SetWeaponInRange`
  (params (WeaponRef :type "/Game/Blueprints/Actors/Weapon Object Reference"))
  (set `self.WeaponToPickUp` WeaponRef)
  (set `self.InRangeOfWeapon` true))

(fn `ThrowWeapon`
  (bind (_returnvalue_x _returnvalue_y _returnvalue_z) (`KismetMathLibrary.BreakVector` (`self.K2_GetActorLocation`)))
  (bind _returnvalue (`|SpawnActorFromClass` "/Game/Blueprints/Actors/Weapon.Weapon_C" (`KismetMathLibrary.MakeTransform` (`KismetMathLibrary.MakeVector` _returnvalue_x _returnvalue_y _returnvalue_z)) "Undefined" "OverrideRootScale" null (`self.WeaponEquipped`) (`self.WeaponData`) null))
  (set `self.WeaponEquipped` "NewEnumerator0")
  (bind _unit_vec (`self.GetLineFromCharToMouse`))
  (`PrimitiveComponent.AddImpulse` (`/Game/Blueprints/Actors/Weapon.Weapon` _returnvalue) (* _unit_vec 500.0) "None" true))

(fn `UserConstructionScript`)

(fn `WeaponOutOfRange`
  (params (WeaponRef :type "/Game/Blueprints/Actors/Weapon Object Reference"))
  (if (== WeaponRef (`self.WeaponToPickUp`))
    (set `self.WeaponToPickUp` null)
    (set `self.InRangeOfWeapon` false)))