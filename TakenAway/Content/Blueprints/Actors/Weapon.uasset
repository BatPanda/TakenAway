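; Weapon is a world pickup actor that shows a Paper2D sprite chosen in the construction script from its Type (fist, knife, shotgun or dev pistol).
; On BeginPlay it gives the sprite a random yaw while keeping its pitch and roll.
; Its Sphere overlap events tell TakenMainCharacter when the weapon enters or leaves range.
; Tick only prints a constant zero, apparently leftover debug output.
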(event `self.ReceiveBeginPlay`
  (bind _weapon (`self.Weapon`))
  (bind (_returnvalue_roll _returnvalue_pitch) (`KismetMathLibrary.BreakRotator` (`SceneComponent.K2_GetComponentRotation` _weapon)))
  (`SceneComponent.K2_SetWorldRotation` _weapon (`KismetMathLibrary.MakeRotator` _returnvalue_roll _returnvalue_pitch (`KismetMathLibrary.RandomFloatInRange` 0.0 359.0)) false false))

(event `self.Sphere.OnComponentBeginOverlap`
  (params (OverlappedComponent :type "PrimitiveComponent Object Reference") (OtherActor :type "Actor Object Reference") (OtherComp :type "PrimitiveComponent Object Reference") (OtherBodyIndex :type Integer) (bFromSweep :type Boolean) (SweepResult :type "HitResult Structure (by ref)"))
  (bind _astaken_main_character (cast `/Game/Blueprints/Actors/TakenMainCharacter` OtherActor))
  (`/Game/Blueprints/Actors/TakenMainCharacter.SetWeaponInRange` _astaken_main_character self))

(event `self.Sphere.OnComponentEndOverlap`
  (params (OverlappedComponent :type "PrimitiveComponent Object Reference") (OtherActor :type "Actor Object Reference") (OtherComp :type "PrimitiveComponent Object Reference") (OtherBodyIndex :type Integer))
  (bind _astaken_main_character (cast `/Game/Blueprints/Actors/TakenMainCharacter` OtherActor))
  (`/Game/Blueprints/Actors/TakenMainCharacter.WeaponOutOfRange` _astaken_main_character self))

(event `self.ReceiveTick`
  (params (DeltaSeconds :type "Float (single-precision)"))
  (`KismetSystemLibrary.PrintString` (`KismetStringLibrary.Conv_DoubleToString` 0.0)))

(fn `UserConstructionScript`
  (`PaperSpriteComponent.SetSprite` (`self.Weapon`) (select `/Game/Blueprints/Core/Weapons` (`self.Type`) :`NewEnumerator1` "/Game/Sprites/Texture_Knife_Side_Sprite.Texture_Knife_Side_Sprite" :`NewEnumerator2` "/Game/Sprites/Texture_Shotgun_Side_Sprite.Texture_Shotgun_Side_Sprite" :`NewEnumerator3` "/Game/Sprites/Dev/Dev_Gun.Dev_Gun" :!type "PaperSprite Object Reference")))