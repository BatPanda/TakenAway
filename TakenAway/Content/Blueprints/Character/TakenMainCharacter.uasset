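; Player character for a top-down game with separate leg and body visuals, moved along world X and Y by axis input.
; Each Tick derives IsMoving from the move axes, then uses it to select the leg sprite's flipbook, with Walking when moving and no idle flipbook assigned.
; The body yaws toward the cursor's Visibility trace hit, independently of movement, with a -90 degree roll offset.
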(event `InputAxis|MoveForward`
  (params (AxisValue :type "Float (single-precision)"))
  (set `self.IsMoving` false)
  (`self.AddMovementInput` (1.0 0.0 0.0) AxisValue)
  (set `self.IsMoving` false))

(event `InputAxis|MoveRight`
  (params (AxisValue :type "Float (single-precision)"))
  (set `self.IsMoving` false)
  (`self.AddMovementInput` (0.0 1.0 0.0) AxisValue)
  (set `self.IsMoving` false))

(event `self.ReceiveTick`
  (params (DeltaSeconds :type "Float (single-precision)"))
  (`self.MovementUpdate`)
  (`self.HandleSprites`))

(fn `BodyMovement`
  (bind (_returnvalue_roll _returnvalue_pitch) (`KismetMathLibrary.BreakRotator` (`self.K2_GetActorRotation`)))
  (bind (_returnvalue_roll_2 _returnvalue_pitch_2 _returnvalue_yaw) (`KismetMathLibrary.BreakRotator` (`KismetMathLibrary.FindLookAtRotation` (`self.K2_GetActorLocation`) (`.Location` (`GameplayStatics.BreakHitResult` (`PlayerController.GetHitResultUnderCursorByChannel` (`GameplayStatics.GetPlayerController` 0) "TraceTypeQuery1" true))))))
  (`SceneComponent.K2_SetWorldRotation` (`self.Body`) (`KismetMathLibrary.MakeRotator` (- _returnvalue_roll 90.0) _returnvalue_pitch _returnvalue_yaw) false false))

(fn `HandleSprites`
  (`self.LegMovement`)
  (`self.BodyMovement`))

(fn `LegMovement`
  (`PaperFlipbookComponent.SetFlipbook` (`self.Sprite`) (select `bool` (`self.IsMoving`) :`true` "/Game/Sprites/Walking.Walking" :!type "PaperFlipbook Object Reference")))

(fn `MovementUpdate`
  (if (and (== (`self.GetInputAxisValue`) 0.0) (== (`self.GetInputAxisValue`) 0.0))
    (set `self.IsMoving` false)
    (else
      (set `self.IsMoving` true))))

(fn `UserConstructionScript`)